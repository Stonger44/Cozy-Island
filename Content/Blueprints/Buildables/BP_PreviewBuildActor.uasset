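; BP_PreviewBuildActor is the placement preview shown for the currently selected buildable.
; ChangePreviewMesh copies the build mesh, rotation and scale from the CurrentBuildableActor class defaults onto SMBuildMesh, so no buildable instance is needed.
; SwapValidInvalidMaterial sets the preview's first material slot to the valid or invalid material based on IsValidSpawn, which this graph only reads.
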(event Custom|ChangePreviewMesh
  (bind _sm_buildmesh (Variables|Default|GetSM_BuildMesh))
  (bind _currentbuildableactor (Variables|Default|GetCurrentBuildableActor))
  (bind (_buildrotation _buildscale _buildmesh) (Utilities|GetClassDefaults _currentbuildableactor))
  (Transformation|SetRelativeRotation _sm_buildmesh _buildrotation false false)
  (Transformation|SetWorldScale3D _sm_buildmesh _buildscale)
  (Components|StaticMesh|SetStaticMesh _sm_buildmesh _buildmesh))

(event Custom|SwapValidInvalidMaterial
  (if (Variables|Default|GetbIsValidSpawn)
    (Rendering|Material|SetMaterial (Variables|Default|GetSM_BuildMesh) 0 (Variables|Default|GetValidMaterial))
    (else
      (Rendering|Material|SetMaterial (Variables|Default|GetSM_BuildMesh) 0 (Variables|Default|GetInvalidMaterial)))))

(fn ConstructionScript)