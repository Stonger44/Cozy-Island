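; BP_Campfire is a buildable campfire that the player can light and put out by interacting with it.
; Interact alternates through a FlipFlop between lighting, which activates the Niagara fire and fades in its audio, and extinguishing, which stops both and plays a fading fizzle.
; Highlight and RemoveHighlight set and clear an overlay material on the campfire mesh to show interaction focus.
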(event EventHighlight
  (Rendering|Material|SetOverlayMaterial (Variables|Default|GetCampfire) (Variables|Default|GetInteractHighlight) :!class /Script/Engine.MeshComponent))

(event EventRemoveHighlight
  (Rendering|Material|SetOverlayMaterial (Variables|Default|GetCampfire) 0 :!class /Script/Engine.MeshComponent))

(event EventInteract
  (bind _audio_fizzle (Variables|Default|GetAudio_Fizzle))
  (bind _audio_fizzle_2 (Variables|Default|GetAudio_Fizzle))
  (Utilities|FlowControl|FlipFlop
    (:A
      (if (Audio|Components|Audio|IsPlaying _audio_fizzle_2)
        (Audio|Components|Audio|Stop _audio_fizzle_2))
      (Components|Activation|Activate (Variables|Default|GetNS_Fire) false)
      (Audio|Components|Audio|FadeIn (Variables|Default|GetAudio_Fire) 1.0 1.0 0.0 "Linear" :!class /Script/Engine.AudioComponent))
    (:B
      (Components|Activation|Deactivate (Variables|Default|GetNS_Fire))
      (Audio|Components|Audio|Stop (Variables|Default|GetAudio_Fire))
      (Audio|Components|Audio|Play _audio_fizzle 0.0)
      (Audio|Components|Audio|FadeOut _audio_fizzle 1.5 0.0 "Linear" :!class /Script/Engine.AudioComponent))))

(fn ConstructionScript)