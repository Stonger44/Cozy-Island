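; BP_LightSwitch is an interactable wall switch that toggles an assigned LightFixture and warns at BeginPlay if none is set.
; Highlight and RemoveHighlight apply and clear an overlay material on the casing and switch.
; Interact alternates a timeline forward and in reverse through a FlipFlop to rotate the switch pivot, ignoring input while switching.
; The light toggles when the timeline finishes, which also releases the IsSwitching lock.
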(event EventBeginPlay
  (Utilities|IsValid (Variables|Default|GetLightFixture)
    (:Is%20Not%20Valid
      (Development|PrintString "Light Fixture is null!"))))

(event EventInteract
  (params (Player :type BP%20First%20Person%20Character%20Object%20Reference))
  (if (not (Variables|Default|GetIsSwitching))
    (Variables|Default|SetIsSwitching true)
    (Utilities|FlowControl|FlipFlop
      (:A
        (bind _alpha (Timeline|LightSwitchTimeline Play)
          (:Update
            (Transformation|SetRelativeRotation (Variables|Default|GetSwitchPivot) (Math|Rotator|Lerp(Rotator) "18.000000,0.000000,0.000000" "0, 0, 0" _alpha) false false))
          (:Finished
            (Default|ToggleLight (Variables|Default|GetLightFixture))
            (Variables|Default|SetIsSwitching false))))
      (:B
        (Timeline|LightSwitchTimeline Reverse)))))

(event EventHighlight
  (bind _interacthighlight (Variables|Default|GetInteractHighlight))
  (Rendering|Material|SetOverlayMaterial (Variables|Default|GetCasing) _interacthighlight :!class /Script/Engine.MeshComponent)
  (Rendering|Material|SetOverlayMaterial (Variables|Default|GetSwitch) _interacthighlight :!class /Script/Engine.MeshComponent))

(event EventRemoveHighlight
  (Rendering|Material|SetOverlayMaterial (Variables|Default|GetCasing) 0 :!class /Script/Engine.MeshComponent)
  (Rendering|Material|SetOverlayMaterial (Variables|Default|GetSwitch) 0 :!class /Script/Engine.MeshComponent))

(fn ConstructionScript)