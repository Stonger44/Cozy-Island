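; BP_Door is an interactable hinged door that swings open and closed, with a highlight overlay material and sound effects.
; Highlight and RemoveHighlight set and clear the overlay material on the door.
; Interact alternates through a FlipFlop, playing the open or close sound and running a timeline forward or in reverse to rotate the DoorPivot.
; An IsSwinging flag ignores further interaction until the swing finishes.
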(event EventHighlight
  (Rendering|Material|SetOverlayMaterial (Variables|Default|GetDoor) (Variables|Default|GetInteractHighlight) :!class /Script/Engine.MeshComponent))

(event EventRemoveHighlight
  (Rendering|Material|SetOverlayMaterial (Variables|Default|GetDoor) 0 :!class /Script/Engine.MeshComponent))

(event EventInteract
  (params (Player :type BP%20First%20Person%20Character%20Object%20Reference))
  (if (not (Variables|Default|GetIsSwinging))
    (Variables|Default|SetIsSwinging true)
    (Utilities|FlowControl|FlipFlop
      (:A
        (Audio|Components|Audio|Play (Variables|Default|GetAudio_DoorOpen) 0.0)
        (bind _alpha (Timeline|DoorSwingTimeline Play)
          (:Update
            (Transformation|SetRelativeRotation (Variables|Default|GetDoorPivot) (Math|Rotator|Lerp(Rotator) "0, 0, 0" "0.000000,125.000000,0.000000" _alpha) false false))
          (:Finished
            (Variables|Default|SetIsSwinging false))))
      (:B
        (Audio|Components|Audio|Play (Variables|Default|GetAudio_DoorClose) 0.0)
        (Timeline|DoorSwingTimeline Reverse)))))

(fn ConstructionScript)