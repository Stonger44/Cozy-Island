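; Base interactable resource source that yields a limited number of resource pickups to the player before it is destroyed.
; Each interaction decrements the count and spawns the resource class at a spawn point, passing a toss direction toward the player and a strength scaled by actor size.
; On depletion it updates the player's nearby-interactable array, clears their focus and destroys itself.
; Highlight events toggle an overlay material on the mesh.
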(event EventBeginPlay
  (Variables|Default|SetResourceCount (Variables|Default|GetMaxResourceCount)))

(event EventInteract
  (params (Player :type BP%20First%20Person%20Character%20Object%20Reference))
  (Variables|Default|SetResourceCount (- (Variables|Default|GetResourceCount) 1))
  (Game|SpawnActorfromClass (Variables|Default|GetResourceClass) (Math|Transform|MakeTransform (.Location (Math|Transform|BreakTransform (Transformation|GetWorldTransform (Variables|Default|GetResourceSpawnPoint))))) "Undefined" "MultiplyWithRoot" 0 (Math|Vector|Normalize (- (Transformation|GetActorLocation Player) (Transformation|GetActorLocation))) (* (Math|Vector|VectorLength (Transformation|GetActorScale3D)) 2e+02) 0)
  (Math|Integer|CompareInt (Variables|Default|GetResourceCount)
    (:==
      _)
    (:<
      _))
  (Utilities|Array|RemoveItem (Variables|/Game/FirstPerson/Blueprints/BP_FirstPersonCharacter.BP_FirstPersonCharacter_C|GetNearbyInteractableArray Player) 0)
  (Variables|/Game/FirstPerson/Blueprints/BP_FirstPersonCharacter.BP_FirstPersonCharacter_C|SetFocusedInteractable Player 0)
  (Actor|DestroyActor))

(event EventHighlight
  (Rendering|Material|SetOverlayMaterial (Variables|Default|GetSM_ResourceSourceMesh) (Variables|Default|GetInteractHighlight) :!class /Script/Engine.MeshComponent))

(event EventRemoveHighlight
  (Rendering|Material|SetOverlayMaterial (Variables|Default|GetSM_ResourceSourceMesh) 0 :!class /Script/Engine.MeshComponent))

(fn ConstructionScript)