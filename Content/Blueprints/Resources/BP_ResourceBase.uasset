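; Base actor for a spinning resource pickup that is tossed to a destination on spawn and collected by the player.
; BeginPlay picks a random mesh and launches the physics driver along a computed arc to TossDestination; an overlap on the resource collision stops the simulation.
; Interacting, or first-person character overlap outside its InteractZone, updates that player's resource count and destroys the actor.
; An overlay material provides the interaction highlight.
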(event OnComponentBeginOverlap(SM_Resource)
  (params (OverlappedComponent :type Primitive%20Component%20Object%20Reference) (OtherActor :type Actor%20Object%20Reference) (OtherComp :type Primitive%20Component%20Object%20Reference) (OtherBodyIndex :type Integer) (bFromSweep :type Boolean) (SweepResult :type Hit%20Result%20Structure%20%28by%20ref%29))
  (bind _asbp_first_person_character (Utilities|Casting|CastToBP_FirstPersonCharacter OtherActor))
  (if (!= (Variables|/Game/FirstPerson/Blueprints/BP_FirstPersonCharacter.BP_FirstPersonCharacter_C|GetInteractZone _asbp_first_person_character) OtherComp)
    (CallFunction|AcquireResource _asbp_first_person_character)))

(event OnComponentBeginOverlap(ResourceCollision)
  (params (OverlappedComponent :type Primitive%20Component%20Object%20Reference) (OtherActor :type Actor%20Object%20Reference) (OtherComp :type Primitive%20Component%20Object%20Reference) (OtherBodyIndex :type Integer) (bFromSweep :type Boolean) (SweepResult :type Hit%20Result%20Structure%20%28by%20ref%29))
  (Physics|SetSimulatePhysics (Variables|Default|GetPhysicsDriver) false))

(event EventBeginPlay
  (Components|StaticMesh|SetStaticMesh (Variables|Default|GetSM_Resource) (.OutItem (Utilities|Array|Random (Variables|Default|GetStaticMeshArray))))
  (bind _outlaunchvelocity (Game|SuggestProjectileVelocityCustomArc (Transformation|GetActorLocation) (Variables|Default|GetTossDestination) 0.0 0.5))
  (Physics|AddImpulse (Variables|Default|GetPhysicsDriver) _outlaunchvelocity "None" true))

(event EventRemoveHighlight
  (Rendering|Material|SetOverlayMaterial (Variables|Default|GetSM_Resource) 0 :!class /Script/Engine.MeshComponent))

(event EventTick
  (params (DeltaSeconds :type Float%20%28single-precision%29))
  (Transformation|AddLocalRotation (Variables|Default|GetRotationPivot) (Math|Rotator|MakeRotator 0.0 0.0 (* DeltaSeconds (Variables|Default|GetRotationSpeed))) false false))

(event EventHighlight
  (Rendering|Material|SetOverlayMaterial (Variables|Default|GetSM_Resource) (Variables|Default|GetInteractHighlight) :!class /Script/Engine.MeshComponent))

(event EventInteract
  (params (Player :type BP%20First%20Person%20Character%20Object%20Reference))
  (CallFunction|AcquireResource Player))

(fn ConstructionScript)

(fn AcquireResource
  (params (Player :type BP%20First%20Person%20Character%20Object%20Reference))
  (Default|UpdateResourceCount Player self)
  (Actor|DestroyActor))