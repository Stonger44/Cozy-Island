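; BP_Resource_Stone is a stone resource pickup, collected either through Interact or by overlapping its mesh with any player component other than InteractZone.
; Both paths call AcquireResource, which increments and prints the player's stone count.
; If listed among the player's nearby interactables, it removes itself, updates the nearby flag, clears focus and destroys itself.
; An unlisted stone still adds to the count but stays in the world.
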(event OnComponentBeginOverlap(SM_ResourceMesh)
  (params (OverlappedComponent :type Primitive%20Component%20Object%20Reference) (OtherActor :type Actor%20Object%20Reference) (OtherComp :type Primitive%20Component%20Object%20Reference) (OtherBodyIndex :type Integer) (bFromSweep :type Boolean) (SweepResult :type Hit%20Result%20Structure%20%28by%20ref%29))
  (bind _asbp_first_person_character (Utilities|Casting|CastToBP_FirstPersonCharacter OtherActor))
  (if (!= (Variables|/Game/FirstPerson/Blueprints/BP_FirstPersonCharacter.BP_FirstPersonCharacter_C|GetInteractZone _asbp_first_person_character) OtherComp)
    (CallFunction|AcquireResource _asbp_first_person_character)))

(event EventInteract
  (params (Player :type BP%20First%20Person%20Character%20Object%20Reference))
  (CallFunction|AcquireResource Player))

(fn ConstructionScript)

(fn AcquireResource
  (params (Player :type BP%20First%20Person%20Character%20Object%20Reference))
  (bind _self self)
  (bind _nearbyinteractablearray (Variables|/Game/FirstPerson/Blueprints/BP_FirstPersonCharacter.BP_FirstPersonCharacter_C|GetNearbyInteractableArray Player))
  (bind _output_get (Variables|/Game/FirstPerson/Blueprints/BP_FirstPersonCharacter.BP_FirstPersonCharacter_C|SetStoneResourceCount Player (+ (Variables|/Game/FirstPerson/Blueprints/BP_FirstPersonCharacter.BP_FirstPersonCharacter_C|GetStoneResourceCount Player) 1)))
  (Development|PrintString (Utilities|String|Append "Stone Resources: " (Utilities|String|ToString(Integer) _output_get)))
  (if (Utilities|Array|ContainsItem _nearbyinteractablearray _self)
    (Utilities|Array|RemoveItem _nearbyinteractablearray _self)
    (Math|Integer|CompareInt (Utilities|Array|Length _nearbyinteractablearray)
      (:>
        _)
      (:==
        (Variables|/Game/FirstPerson/Blueprints/BP_FirstPersonCharacter.BP_FirstPersonCharacter_C|SetbIsInteractableNearby Player false :!label _label))
      (:<
        (goto _label)))
    (Variables|/Game/FirstPerson/Blueprints/BP_FirstPersonCharacter.BP_FirstPersonCharacter_C|SetFocusedInteractable Player 0)
    (Actor|DestroyActor)))