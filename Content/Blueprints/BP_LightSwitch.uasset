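; BP_LightSwitch is an interactable light switch with Casing and Switch meshes and a reference to a LightFixture.
; On BeginPlay it prints a warning if the LightFixture reference is not valid.
; Highlight and RemoveHighlight set and clear the InteractHighlight overlay material on both meshes.
; The Interact event is an empty stub, so the switch does not yet control the fixture.
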(event EventBeginPlay
  (Utilities|IsValid (Variables|Default|GetLightFixture)
    (:Is%20Not%20Valid
      (Development|PrintString "Light Fixture is null!"))))

(event EventInteract)

(event EventHighlight
  (bind _interacthighlight (Variables|Default|GetInteractHighlight))
  (Rendering|Material|SetOverlayMaterial (Variables|Default|GetCasing) _interacthighlight :!class /Script/Engine.MeshComponent)
  (Rendering|Material|SetOverlayMaterial (Variables|Default|GetSwitch) _interacthighlight :!class /Script/Engine.MeshComponent))

(event EventRemoveHighlight
  (Rendering|Material|SetOverlayMaterial (Variables|Default|GetCasing) 0 :!class /Script/Engine.MeshComponent)
  (Rendering|Material|SetOverlayMaterial (Variables|Default|GetSwitch) 0 :!class /Script/Engine.MeshComponent))

(fn ConstructionScript)