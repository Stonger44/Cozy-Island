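; BP_Tool_Pickup is a tool pickup actor that the player collects by interacting with it or touching it.
; Highlight and RemoveHighlight set and clear an overlay material on the tool mesh.
; Both Interact and mesh overlap pass the pickup to the player's UpdateToolBool, then destroy it.
; The overlap path accepts only BP_FirstPersonCharacter and ignores its InteractZone component, so that zone alone does not trigger collection.
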(event OnComponentBeginOverlap(SM_Tool)
  (params (OverlappedComponent :type Primitive%20Component%20Object%20Reference) (OtherActor :type Actor%20Object%20Reference) (OtherComp :type Primitive%20Component%20Object%20Reference) (OtherBodyIndex :type Integer) (bFromSweep :type Boolean) (SweepResult :type Hit%20Result%20Structure%20%28by%20ref%29))
  (bind _asbp_first_person_character (Utilities|Casting|CastToBP_FirstPersonCharacter OtherActor))
  (if (!= (Variables|/Game/FirstPerson/Blueprints/BP_FirstPersonCharacter.BP_FirstPersonCharacter_C|GetInteractZone _asbp_first_person_character) OtherComp)
    (Default|UpdateToolBool _asbp_first_person_character self)
    (Actor|DestroyActor)))

(event EventInteract
  (params (Player :type BP%20First%20Person%20Character%20Object%20Reference))
  (Default|UpdateToolBool Player self)
  (Actor|DestroyActor))

(event EventHighlight
  (Rendering|Material|SetOverlayMaterial (Variables|Default|GetSM_Tool) (Variables|Default|GetInteractHighlight) :!class /Script/Engine.MeshComponent))

(event EventRemoveHighlight
  (Rendering|Material|SetOverlayMaterial (Variables|Default|GetSM_Tool) 0 :!class /Script/Engine.MeshComponent))

(fn ConstructionScript)