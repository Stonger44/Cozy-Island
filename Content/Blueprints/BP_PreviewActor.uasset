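; BP_PreviewActor is a placement preview actor that shows a mesh and signals whether the spawn spot is valid.
; Its events apply the stored collision type and current mesh to the SMPreviewMesh component.
; Material slot 0 switches between valid and invalid materials based on IsValidSpawn, or takes an indexed entry from a default materials array.
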(event Custom|ChangePreviewMesh
  (Components|StaticMesh|SetStaticMesh (Variables|Default|GetSM_PreviewMesh) (Variables|Default|GetCurrentMesh)))

(event Custom|SwapValidInvalidMaterial
  (if (Variables|Default|GetbIsValidSpawn)
    (Rendering|Material|SetMaterial (Variables|Default|GetSM_PreviewMesh) 0 (Variables|Default|GetValidMaterial))
    (else
      (Rendering|Material|SetMaterial (Variables|Default|GetSM_PreviewMesh) 0 (Variables|Default|GetInvalidMaterial)))))

(event Custom|ChangeCollisionType
  (Collision|SetCollisionEnabled (Variables|Default|GetSM_PreviewMesh) (Variables|Default|GetCollisionType)))

(event Custom|SetDefaultMaterial
  (Rendering|Material|SetMaterial (Variables|Default|GetSM_PreviewMesh) 0 (Utilities|Array|Get(acopy) (Variables|Default|GetDefaultMaterials) (Variables|Default|GetDefaultMaterialIndex))))

(fn ConstructionScript)