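; BP_Door is an interactable door that swings open and closed and can show a highlight.
; Interact alternates through a FlipFlop, playing the matching sound and running a timeline forward or in reverse to rotate the DoorPivot.
; An IsSwinging flag ignores interaction until the timeline finishes.
; Highlight and RemoveHighlight set and clear an overlay material on the door mesh.
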(event EventHighlight
  (Rendering|Material|SetOverlayMaterial (Variables|Default|GetDoor) (Variables|Default|GetInteractHighlight) :!class /Script/Engine.MeshComponent))

(event EventRemoveHighlight
  (Rendering|Material|SetOverlayMaterial (Variables|Default|GetDoor) 0 :!class /Script/Engine.MeshComponent))

(event EventInteract
  (if (not (Variables|Default|GetIsSwinging))
    (Variables|Default|SetIsSwinging true)
    (bind _isa (Utilities|FlowControl|FlipFlop)
      (:A
        _)
      (:B
        _))
    (if _isa
      (Audio|Components|Audio|Play (Variables|Default|GetAudio_DoorOpen) 0.0)
      (bind _alpha (Timeline|OpenDoorTimeline Play)
        (:Update
          (Transformation|SetRelativeRotation (Variables|Default|GetDoorPivot) (Math|Rotator|Lerp(Rotator) "0, 0, 0" "0.000000,125.000000,0.000000" _alpha) false false))
        (:Finished
          (Variables|Default|SetIsSwinging false)))
      (else
        (Audio|Components|Audio|Play (Variables|Default|GetAudio_DoorClose) 0.0)
        (Timeline|OpenDoorTimeline Reverse)))))

(fn ConstructionScript)